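; Base door Blueprint, apparently an unfinished scaffold for a lockable door that the player character can interact with.
; InteractPlayerCharacter only stores the player reference and reassigns IsLocked to itself; construction and event entry points are empty.
; Disconnected fragments sketch a collision-disabling timeline, a locked message and player-relative swing direction math, but none of them run.
; Open speed, angle and state variables are not yet used by live logic.
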(fn `InteractPlayerCharacter`
  (params (PlayerCharacter :type "CharacterEvent Structure"))
  (locals (NewLocalVar :type "Actor Object Reference"))
  (set `self.PlayerRef` PlayerCharacter)
  (set `self.Is Locked` (`self.IsLocked`)))

(fn `UserConstructionScript`)