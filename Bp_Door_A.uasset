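; Door actor that swings open automatically when the third-person character enters its trigger box and closes when they leave.
; Box overlap events play or reverse a timeline, whose alpha drives the door frame's relative yaw up to a quarter turn.
; An interact and open/closed toggle system is left unfinished: its functions are empty stubs or disconnected nodes, so only the overlap logic moves the door.
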(event `self.Boxforframe.OnComponentBeginOverlap`
  (params (OverlappedComponent :type "PrimitiveComponent Object Reference") (OtherActor :type "Actor Object Reference") (OtherComp :type "PrimitiveComponent Object Reference") (OtherBodyIndex :type Integer) (bFromSweep :type Boolean) (SweepResult :type "HitResult Structure (by ref)"))
  (cast `/Game/TPAA_/Blueprints/BP_ThirdPersonCharacter` OtherActor)
  (bind (_direction _alpha) (`Timeline|DoorTimeLine` :!label _label)
    (:`Update`
      (`SceneComponent.K2_SetRelativeRotation` (`self.doorframe`) (`KismetMathLibrary.MakeRotator` 0.0 0.0 (* _alpha 90.0)) false false))))

(event `self.Boxforframe.OnComponentEndOverlap`
  (params (OverlappedComponent :type "PrimitiveComponent Object Reference") (OtherActor :type "Actor Object Reference") (OtherComp :type "PrimitiveComponent Object Reference") (OtherBodyIndex :type Integer))
  (cast `/Game/TPAA_/Blueprints/BP_ThirdPersonCharacter` OtherActor)
  (goto _label :!via `Reverse`))

(event `self.ReceiveBeginPlay`)

(event `CloseDoor`)

(fn `interact`
  (params (InteractActor :type "Character Object Reference") (`Interact Character` :type Boolean))
  (returns (Success :type Boolean))
  (locals (NewLocalVar :type "Actor Object Reference")))

(fn `return node`
  (params (Success :type Boolean)))

(fn `SwitchDoorOpen`)

(fn `UpdateDoorVisual`)

(fn `UserConstructionScript`)