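; Door Blueprint child that adds a lock state, lock icons and a rotation feedback for trying a locked door.
; UpdateDoorVisual branches on Bisdoorlocked: true calls the parent, false plays the locked-feedback timeline, which yaws the door by angle and CurrentDotProduct.
; Construction sets back icon visibility from the flag, and the open-on-construct override derives IsdoorOpen from it.
; UnLockDoor clears the flag, swaps both icons to open-lock meshes and updates their visibility.
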(event `TryOpenLockedDoor`
  (bind (_direction _doorlockedtryingprogress) (`Timeline|LockedFeedbackTimeline`)
    (:`Update`
      (`SceneComponent.K2_SetRelativeRotation` (`self.DoorScene`) (`KismetMathLibrary.MakeRotator` 0.0 0.0 (* (`self.LockedDoorAnglee`) _doorlockedtryingprogress (`self.Current Dot Product`))) false false))))

(fn `ConfigureOpenDoorOnConstruct`
  (set `self.bIsdoorOpen` (not (`self.bisdoorlocked`)))
  (`parent.ConfigureOpenDoorOnConstruct`))

(fn `UnLockDoor`
  (set `self.bisdoorlocked` false)
  (`self.UnLockFeedback`))

(fn `UnLockFeedback`
  (`StaticMeshComponent.SetStaticMesh` (`self.Icon__LockedClosedMeshF`) "/Game/Polygon_Prototype/Meshes/Icons/SM_Icon_Lock_Open_01.SM_Icon_Lock_Open_01")
  (`StaticMeshComponent.SetStaticMesh` (`self.Icon__LockedClosedMeshB`) "/Game/Polygon_Prototype/Meshes/Icons/SM_Icon_Lock_Open_01.SM_Icon_Lock_Open_01")
  (`KismetSystemLibrary.K2_SetTimer` null "" 2.0)
  (`SceneComponent.SetVisibility` (`self.Icon__LockedClosedMeshB`) (`self.bisdoorlocked`) false)
  (`SceneComponent.SetVisibility` (`self.Icon__LockedClosedMeshF`) (`self.bisdoorlocked`) false))

(fn `UpdateDoorVisual`
  (if (`self.bisdoorlocked`)
    (`parent.UpdateDoorVisual`)
    (else
      (`self.TryOpenLockedDoor`))))

(fn `UserConstructionScript`
  (`parent.UserConstructionScript`)
  (`SceneComponent.SetVisibility` (`self.Icon__LockedClosedMeshB`) (`self.bisdoorlocked`) false))